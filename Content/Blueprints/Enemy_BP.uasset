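; Enemy character for a Pac-Man style game that chases the player pawn with AI movement.
; A bound state-change event drives movement: Hunt follows the player, Idle stops, Run Away returns to the start position.
; It starts hunting after a short idle.
; Touching a powered-up Pacman teleports it to the center to resume hunting later; otherwise it banishes Pacman off-map and reloads Level_01 after a delay.
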(event `Event State Changed Setup`
  (add `self.StateChangedEvent` (delegate `Event State Changed`)))

(event `Event State Changed` :!signature `self.StateChangedEvent`
  (params (NewState :type "EEnemyState Enum" :default "Hunt"))
  (`KismetSystemLibrary.PrintString` (`|GetEnumeratorNameAsString` NewState))
  (`self.Update Movement Target`) ; プレイヤー追尾
)

(event `self.ReceiveBeginPlay`
  (`self.Event State Changed Setup`)
  (`self.Idle`) ; 待機
  (`KismetSystemLibrary.Delay` 1.5) ; 1.5秒後に
  (`self.Hunt`) ; 追いかける
)

(event `self.Sphere.OnComponentHit`
  (params (HitComponent :type "PrimitiveComponent Object Reference") (OtherActor :type "Actor Object Reference") (OtherComp :type "PrimitiveComponent Object Reference") (NormalImpulse :type "Vector Structure") (Hit :type "HitResult Structure (by ref)"))
  (bind _aspacman_bp (cast `/Game/Blueprints/Pacman_BP` OtherActor)) ; プレイヤーに接触
  (bind _returnvalue (`PacmanPawn.IsPowerUp` _aspacman_bp)) ; プレイヤーがパワーアップ時
  (if _returnvalue
    (`self.K2_SetActorLocation` (0.0 100.0 0.0)) ; 敵は中央に
    (`KismetSystemLibrary.Delay` 1.5) ; 1.5秒後に
    (`self.Hunt`) ; 追いかける
    (else
      (`self.K2_SetActorLocation` _aspacman_bp (10000.0 10000.0 10000.0) false false) ; プレイヤー消滅
      (`self.Idle`) ; 敵は待機
      (`KismetSystemLibrary.Delay` 2.0) ; 2秒後に
      (`GameplayStatics.OpenLevel` "Level_01") ; 遷移
    )))

(fn `Death Movement`
  (locals (EnemyStartPos :type "Vector Structure" :default (0.0 100.0 0.0)))
  (set `self.AI Controller` (`AIBlueprintHelperLibrary.GetAIController` (`self.GetController`)))
  (`AIBlueprintHelperLibrary.SimpleMoveToLocation` (`self.AI Controller`) (`local.EnemyStartPos`)) ; 初期位置に戻る
)

(fn `Update Movement Target`
  (bind _returnvalue (`AIBlueprintHelperLibrary.GetAIController` (`self.GetController`)))
  (switch `EEnemyState` (`self.State`)
    (:`Hunt`
      (`AIController.MoveToActor` _returnvalue (`GameplayStatics.GetPlayerPawn` 0) 0.0 false true true null true))
    (:`Idle`
      (`Controller.StopMovement` _returnvalue))
    (:`RunAway`
      (`self.Death Movement`))))

(fn `UserConstructionScript`)